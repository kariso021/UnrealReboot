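; BPC_Attacks is an actor component providing reusable attacks for its owning character: bullets, melee swings, ground smash, leaping strikes and magic projectiles.
; Most attacks play a montage, fire hits on its notifies and message the owner about attack end and, for some, interruptibility.
; Traces and spawned AOE actors filter damage by team number, while projectiles damage on impact.
; Leaps launch toward the target's predicted position with a distance-scaled arc.
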(event `FireBullet`
  (params (TraceStart :type "Vector Structure") (TraceEnd :type "Vector Structure") (DamageInfo :type "FallbackStruct Structure"))
  ;[1 1 1] Attack Notifies
  (bind (_outhits _returnvalue) (`KismetSystemLibrary.LineTraceMultiForObjects` TraceStart TraceEnd (`|MakeArray` "ObjectTypeQuery3" :!type "EObjectTypeQuery Enum") false (`|MakeArray` (`self.GetOwner`))))
  (if _returnvalue
    (bind _damagedactor (`self.DamageFirstNonTeamMember` _outhits DamageInfo))
    (`AISense_Damage.ReportDamageEvent` _damagedactor (`self.GetOwner`) (`.Amount_2_64864A0D4320D27C3EA14D8019B5EC9D` (break `FallbackStruct` DamageInfo)) (`Actor.K2_GetActorLocation` (`self.GetOwner`)))))

(event `GroundSmash`
  (params (AttackInfo :type "/Game/Attacks/S_AttackInfo Structure") (Radius :type "Float (single-precision)"))
  (bind (_attacktarget _montage _damageinfo) (break `/Game/Attacks/S_AttackInfo` AttackInfo))
  (bind _returnvalue (`self.GetOwner`))
  (bind _mesh (`self.AttackBase` _attacktarget))
  (bind _notifyname (`|PlayMontage` _mesh _montage)
    (:`then`
      (message `/Game/Attacks/BPC_Attacks.SetIsInterruptible` _returnvalue false))
    (:`OnCompleted`
      (message `/Game/Attacks/BPC_Attacks.AttackEnd` _returnvalue _attacktarget :!label _label)
      (message `/Game/Attacks/BPC_Attacks.SetIsInterruptible` _returnvalue true))
    (:`OnInterrupted`
      (goto _label))
    (:`OnNotifyBegin`
      (switch `name` _notifyname
        (:`Smash`
          (`self.AOEDamage` Radius _damageinfo))))))

(event `MagicSpell`
  (params (SpawnTransform :type "Transform Structure") (Target :type "Actor Object Reference") (DamageInfo :type "FallbackStruct Structure") (Alt :type Boolean))
  ;[1 1 1] Attack Notifies
  (bind _returnvalue (`|SpawnActorFromClass` (select `bool` Alt :`false` "/Game/Projectiles/BP_Projectile_DarkEnergy.BP_Projectile_DarkEnergy_C" :`true` "/Game/Projectiles/BP_Projectile_DarkEnergy_Alt.BP_Projectile_DarkEnergy_Alt_C" :!type "/Game/Projectiles/BP_Projectile_Base Class Reference") SpawnTransform "Undefined" "MultiplyWithRoot" (`self.GetOwner`) 1000.0 0.0 Target false null))
  (add `/Game/Projectiles/BP_Projectile_Base.OnProjectileImpact` _returnvalue (delegate `OnProjectileHit`))
  (`PrimitiveComponent.IgnoreActorWhenMoving` (`Actor.GetComponentByClass` (`self.GetOwner`) "/Script/Engine.CapsuleComponent") _returnvalue true))

(event `PrimaryMeleeAttack`
  (params (AttackInfo :type "/Game/Attacks/S_AttackInfo Structure") (Radius :type "Float (single-precision)") (Length :type "Float (single-precision)"))
  (bind (_attacktarget _montage _damageinfo) (break `/Game/Attacks/S_AttackInfo` AttackInfo))
  (bind _mesh (`self.AttackBase` _attacktarget))
  (bind _notifyname (`|PlayMontage` _mesh _montage)
    (:`OnCompleted`
      (message `/Game/Attacks/BPC_Attacks.AttackEnd` (`self.GetOwner`) _attacktarget :!label _label_2))
    (:`OnInterrupted`
      (goto _label_2))
    (:`OnNotifyBegin`
      (switch `name` _notifyname
        (:`Slash`
          (`self.SphereTraceDamage` _damageinfo Radius Length))))))

(event `OnProjectileHit`
  (params (OtherActor :type "Actor Object Reference") (Hit :type "HitResult Structure"))
  (bind _returnvalue (`self.GetOwner`))
  ;[1 1 1] Attack Notifies
  (message `/Game/Attacks/BPC_Attacks.TakeDamage` OtherActor (stale `MagicSpell` DamageInfo) _returnvalue)
  (`AISense_Damage.ReportDamageEvent` OtherActor _returnvalue (`.Amount_2_64864A0D4320D27C3EA14D8019B5EC9D` (break `FallbackStruct` (stale `MagicSpell` DamageInfo))) (`Actor.K2_GetActorLocation` (`self.GetOwner`)))
  (`self.OnAttackEnded`))

(event `LongRangeMeleeAttack`
  (params (AttackInfo :type "/Game/Attacks/S_AttackInfo Structure"))
  (bind (_attacktarget _montage _damageinfo) (break `/Game/Attacks/S_AttackInfo` AttackInfo))
  (bind _returnvalue (`self.GetOwner`))
  (bind _mesh (`self.AttackBase` _attacktarget))
  (bind _notifyname (`|PlayMontage` _mesh _montage)
    (:`then`
      (message `/Game/Attacks/BPC_Attacks.SetIsInterruptible` _returnvalue false))
    (:`OnCompleted`
      (message `/Game/Attacks/BPC_Attacks.AttackEnd` _returnvalue _attacktarget :!label _label_3)
      (message `/Game/Attacks/BPC_Attacks.SetIsInterruptible` _returnvalue true))
    (:`OnInterrupted`
      (goto _label_3))
    (:`OnNotifyBegin`
      (switch `name` _notifyname
        (:`Slash`
          (`self.SphereTraceDamage` _damageinfo 20.0 200.0))
        (:`Jump`
          (`self.JumpToAttackTarget` _attacktarget))
        (:`AOESlash`
          (`self.AOEDamage` 300.0 _damageinfo))))))

(event `AOEDamage`
  (params (Radius :type "Float (single-precision)") (DamageInfo :type "FallbackStruct Structure"))
  (bind _returnvalue (`self.GetOwner`))
  ;[1 1 1] Attack Notifies
  (bind _returnvalue_2 (`|SpawnActorFromClass` "/Game/AOE/BP_AOE_Base.BP_AOE_Base_C" (`KismetMathLibrary.MakeTransform` (`Actor.K2_GetActorLocation` _returnvalue)) "Undefined" "MultiplyWithRoot" null false true false (cast `Pawn` _returnvalue :!pure true)))
  (set `/Game/AOE/BP_AOE_Base.Radius` Radius _returnvalue_2)
  (add `/Game/AOE/BP_AOE_Base.OnAOEOverlapActor` _returnvalue_2 (delegate `AOEDamageActor`))
  (`/Game/AOE/BP_AOE_Base.Trigger` _returnvalue_2))

(event `AOEDamageActor`
  (params (Actor :type "Actor Object Reference"))
  ;[1 1 1] Attack Notifies
  (bind _teamnumber (message `/Game/Attacks/BPC_Attacks.GetTeamNumber` Actor))
  (bind _teamnumber_2 (message `/Game/Attacks/BPC_Attacks.GetTeamNumber` (`self.GetOwner`)))
  (if (!= _teamnumber_2 _teamnumber)
    (message `/Game/Attacks/BPC_Attacks.TakeDamage` Actor (stale `AOEDamage` DamageInfo) (`self.GetOwner`))))

(event `SphereTraceDamage`
  (params (DamageInfo :type "FallbackStruct Structure") (Radius :type "Float (single-precision)") (Length :type "Float (single-precision)"))
  (bind _returnvalue (`self.GetOwner`))
  (bind _returnvalue_2 (`Actor.K2_GetActorLocation` _returnvalue))
  ;[1 1 1] Attack Notifies
  (bind (_outhits _returnvalue_3) (`KismetSystemLibrary.SphereTraceMultiForObjects` _returnvalue_2 (+ _returnvalue_2 (* (`Actor.GetActorForwardVector` _returnvalue) Length)) Radius (`|MakeArray` "ObjectTypeQuery3" :!type "EObjectTypeQuery Enum")))
  (if _returnvalue_3
    (`self.DamageAllNonTeamMebers` _outhits DamageInfo)))

(event `SpinningMeleeAttack`
  (params (AttackInfo :type "/Game/Attacks/S_AttackInfo Structure"))
  (bind (_attacktarget _montage _damageinfo) (break `/Game/Attacks/S_AttackInfo` AttackInfo))
  (bind _returnvalue (`self.GetOwner`))
  (bind _mesh (`self.AttackBase` _attacktarget))
  (bind _notifyname (`|PlayMontage` _mesh _montage)
    (:`then`
      (message `/Game/Attacks/BPC_Attacks.SetIsInterruptible` _returnvalue false))
    (:`OnCompleted`
      (message `/Game/Attacks/BPC_Attacks.AttackEnd` _returnvalue _attacktarget :!label _label_4)
      (message `/Game/Attacks/BPC_Attacks.SetIsInterruptible` _returnvalue true))
    (:`OnInterrupted`
      (goto _label_4))
    (:`OnNotifyBegin`
      (switch `name` _notifyname
        (:`Slash`
          (`self.SphereTraceDamage` _damageinfo 20.0 200.0))
        (:`AOESlash`
          (`self.AOEDamage` 300.0 _damageinfo))))))

(event `JumpToAttackTarget`
  (params (AttackTarget :type "Actor Object Reference"))
  (bind _ascharacter (cast `Character` (`self.GetOwner`) :!pure true))
  ;[1 1 1] Attack Notifies
  (bind _location (`self.CalculateFutureActorLocation` AttackTarget))
  (bind _outlaunchvelocity (`GameplayStatics.SuggestProjectileVelocity_CustomArc` (`Actor.K2_GetActorLocation` (`self.GetOwner`)) (`KismetMathLibrary.MakeVector` (.x _location) (.y _location) (+ (.z _location) 100.0)) 0.0 (`KismetMathLibrary.Lerp` 0.5 0.94 (`KismetMathLibrary.FClamp` (`KismetMathLibrary.NormalizeToRange` (`Actor.GetDistanceTo` AttackTarget (`self.GetOwner`)) 400.0 800.0)))))
  (`Character.LaunchCharacter` _ascharacter _outlaunchvelocity true true)
  (add `Character.LandedDelegate` _ascharacter (delegate `OnHit`)))

(event `OnHit`
  (params (Hit :type "HitResult Structure (by ref)"))
  (bind _ascharacter (cast `Character` (`self.GetOwner`) :!pure true))
  ;[1 1 1] Attack Notifies
  (remove `Character.LandedDelegate` _ascharacter (delegate `OnHit`))
  (`MovementComponent.StopMovementImmediately` (`Character.CharacterMovement` _ascharacter)))

(event `BasicMageSpell`
  (params (AttackInfo :type "/Game/Attacks/S_AttackInfo Structure"))
  (bind (_attacktarget _montage _damageinfo) (break `/Game/Attacks/S_AttackInfo` AttackInfo))
  (bind _mesh (`self.AttackBase` _attacktarget))
  (bind _notifyname (`|PlayMontage` _mesh _montage)
    (:`OnCompleted`
      (message `/Game/Attacks/BPC_Attacks.AttackEnd` (`self.GetOwner`) _attacktarget :!label _label_5))
    (:`OnInterrupted`
      (goto _label_5))
    (:`OnNotifyBegin`
      (switch `name` _notifyname
        (:`Fire`
          (`self.MagicSpell` (`KismetMathLibrary.MakeTransform` (`SceneComponent.GetSocketLocation` _mesh "RightHand")) _attacktarget _damageinfo))))))

(event `PlayerSpell`
  (params (SpawnTransform :type "Transform Structure") (Target :type "Actor Object Reference") (DamageInfo :type "FallbackStruct Structure") (Alt :type Boolean))
  (bind _returnvalue (`|SpawnActorFromClass` (select `bool` Alt :`false` "/Game/Projectiles/BP_Projectile_DarkEnergy_Alt.BP_Projectile_DarkEnergy_Alt_C" :`true` "/Game/Projectiles/BP_Projectile_DarkEnergy_Alt.BP_Projectile_DarkEnergy_Alt_C" :!type "/Game/Projectiles/BP_Projectile_Base Class Reference") SpawnTransform "Undefined" "MultiplyWithRoot" (`self.GetOwner`) 1000.0 0.0 Target false null))
  ;[1 1 1] Attack Notifies
  (add `/Game/Projectiles/BP_Projectile_Base.OnProjectileImpact` _returnvalue (delegate `CustomEvent_1`))
  (`PrimitiveComponent.IgnoreActorWhenMoving` (`Actor.GetComponentByClass` (`self.GetOwner`) "/Script/Engine.CapsuleComponent") _returnvalue true))

(event `CustomEvent_1`
  (params (OtherActor :type "Actor Object Reference") (Hit :type "HitResult Structure"))
  (bind _returnvalue (`self.GetOwner`))
  (message `/Game/Attacks/BPC_Attacks.TakeDamage` OtherActor (stale `PlayerSpell` DamageInfo) _returnvalue)
  (`AISense_Damage.ReportDamageEvent` OtherActor _returnvalue (`.Amount_2_64864A0D4320D27C3EA14D8019B5EC9D` (break `FallbackStruct` (stale `PlayerSpell` DamageInfo))) (`Actor.K2_GetActorLocation` (`self.GetOwner`)))
  (`self.OnAttackEnded`))

(event `BarrageMagicSpell`
  (params (AttackInfo :type "/Game/Attacks/S_AttackInfo Structure"))
  (bind (_attacktarget _montage _damageinfo) (break `/Game/Attacks/S_AttackInfo` AttackInfo))
  (bind _returnvalue (`self.GetOwner`))
  (bind _mesh (`self.AttackBase` _attacktarget))
  (bind _notifyname (`|PlayMontage` _mesh _montage)
    (:`OnCompleted`
      (message `/Game/Attacks/BPC_Attacks.AttackEnd` _returnvalue _attacktarget :!label _label_6)
      (message `/Game/Attacks/BPC_Attacks.SetIsInterruptible` _returnvalue true))
    (:`OnInterrupted`
      (goto _label_6))
    (:`OnNotifyBegin`
      (switch `name` _notifyname
        (:`Fire`
          (`self.MagicSpell` (`KismetMathLibrary.MakeTransform` (`SceneComponent.GetSocketLocation` _mesh "RightHand") (`KismetMathLibrary.FindLookAtRotation` (`Actor.K2_GetActorLocation` (`self.GetOwner`)) (+ (`Actor.K2_GetActorLocation` _attacktarget) (`KismetMathLibrary.MakeVector` 0.0 (`KismetMathLibrary.RandomFloatInRange` -300.0 300.0))))) null _damageinfo true)
          (message `/Game/Attacks/BPC_Attacks.SetIsInterruptible` _returnvalue false))))))

(fn `AttackBase`
  (params (AttackTarget :type "Actor Object Reference"))
  (returns (Mesh :type "SkeletalMeshComponent Object Reference"))
  (bind _returnvalue (`self.GetOwner`))
  (message `/Game/Attacks/BPC_Attacks.Attack` _returnvalue AttackTarget)
  (bind _ascharacter (cast `Character` _returnvalue))
  (return (`Character.Mesh` _ascharacter)))

(fn `CalculateFutureActorLocation`
  (params (Actor :type "Actor Object Reference") (Time :type "Float (double-precision)" :default 1.0))
  (returns (Location :type "Vector Structure"))
  (return (+ (`Actor.K2_GetActorLocation` Actor) (* (* (`Actor.GetVelocity` Actor) (1.0 1.0 0.0)) Time))))

(fn `DamageAllNonTeamMebers`
  (params (Hits :type "Array of HitResult Structure") (DamageInfo :type "FallbackStruct Structure"))
  (returns (ActorsDamaged :type "Array of Actor Object Reference"))
  (locals (ActorsDamagedSoFar :type "Array of Actor Object Reference"))
  (for _array_element Hits
    (bind (_bblockinghit _binitialoverlap _time _distance _location _impactpoint _normal _impactnormal _physmat _hitactor) (`GameplayStatics.BreakHitResult` _array_element))
    (bind _teamnumber (message `/Game/Attacks/BPC_Attacks.GetTeamNumber` _hitactor))
    (bind _teamnumber_2 (message `/Game/Attacks/BPC_Attacks.GetTeamNumber` (`self.GetOwner`)))
    (if (and (!= _teamnumber_2 _teamnumber) (not (`KismetArrayLibrary.Array_Contains` (`local.ActorsDamagedSoFar`) _hitactor)))
      (message `/Game/Attacks/BPC_Attacks.TakeDamage` _hitactor DamageInfo (`self.GetOwner`))
      (`KismetArrayLibrary.Array_AddUnique` (`local.ActorsDamagedSoFar`) _hitactor)))
  (return (`local.ActorsDamagedSoFar`)))

(fn `DamageFirstNonTeamMember`
  (params (Hits :type "Array of HitResult Structure") (DamageInfo :type "FallbackStruct Structure"))
  (returns (DamagedActor :type "Actor Object Reference"))
  (for _array_element Hits
    (bind (_bblockinghit _binitialoverlap _time _distance _location _impactpoint _normal _impactnormal _physmat _hitactor) (`GameplayStatics.BreakHitResult` _array_element))
    (bind _teamnumber (message `/Game/Attacks/BPC_Attacks.GetTeamNumber` _hitactor))
    (bind _teamnumber_2 (message `/Game/Attacks/BPC_Attacks.GetTeamNumber` (`self.GetOwner`)))
    (if (!= _teamnumber_2 _teamnumber)
      (message `/Game/Attacks/BPC_Attacks.TakeDamage` _hitactor DamageInfo (`self.GetOwner`))
      (`|ExecutionSequence`
        (:`then_0`
          (break))
        (:`then_1`
          (return _hitactor))))))